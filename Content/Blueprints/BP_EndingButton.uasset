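; BP_EndingButton is a level-ending button that opens the next-level screen once the player's button count exceeds one.
; Each capsule overlap by BP_ThirdPersonCharacterCustom increments that character's ButtonCount and sets the Button component visible only above that threshold.
; Above it, W_NextLevel appears with UI-only input and a mouse cursor.
; Otherwise, it hides the button and prints the incremented count plus one.
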(event `self.Capsule.OnComponentBeginOverlap`
  (params (OverlappedComponent :type "PrimitiveComponent Object Reference") (OtherActor :type "Actor Object Reference") (OtherComp :type "PrimitiveComponent Object Reference") (OtherBodyIndex :type Integer) (bFromSweep :type Boolean) (SweepResult :type "HitResult Structure (by ref)"))
  (bind _returnvalue (`GameplayStatics.GetPlayerController` 0))
  (bind _asbp_third_person_character_custom (cast `/Game/Blueprints/BP_ThirdPersonCharacterCustom` OtherActor))
  (bind _returnvalue_2 (+ (`/Game/Blueprints/BP_ThirdPersonCharacterCustom.buttonCount` _asbp_third_person_character_custom) 1))
  (bind _output_get (set `/Game/Blueprints/BP_ThirdPersonCharacterCustom.buttonCount` _returnvalue_2 _asbp_third_person_character_custom))
  (bind _returnvalue_3 (> _output_get 1))
  (`SceneComponent.SetVisibility` (`self.button`) _returnvalue_3 false)
  (if _returnvalue_3
    (bind _returnvalue_4 (`|CreateWidget` "/Game/Widgets/W_NextLevel.W_NextLevel_C"))
    (`UserWidget.AddToViewport` _returnvalue_4 0)
    (`WidgetBlueprintLibrary.SetInputMode_UIOnlyEx` _returnvalue _returnvalue_4)
    (set `PlayerController.bShowMouseCursor` true _returnvalue)
    (else
      (`KismetSystemLibrary.PrintString` (`KismetStringLibrary.Conv_IntToString` _returnvalue_2)))))

(fn `UserConstructionScript`)