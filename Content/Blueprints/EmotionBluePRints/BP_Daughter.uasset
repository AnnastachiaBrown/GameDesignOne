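; BP_Daughter is a collectible child actor that the player picks up by overlapping its Trigger.
; On BeginPlay the KidMoving timeline lerps CustomMesh between the Start and End components, feeding their world locations into a relative-location setter.
; When BP_ThirdPersonCharacterCustom enters the Trigger, it increments that character's KidCount, then destroys itself.
; Debug prints mark the movement updates and the pickup.
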(event `self.ReceiveBeginPlay`
  (bind (_direction _floattrack) (`Timeline|KidMoving` :!via `PlayFromStart`)
    (:`Update`
      (`SceneComponent.K2_SetRelativeLocation` (`self.CustomMesh`) (`KismetMathLibrary.VLerp` (`SceneComponent.K2_GetComponentLocation` (`self.start`)) (`SceneComponent.K2_GetComponentLocation` (`self.end`)) _floattrack) false false)
      (`KismetSystemLibrary.PrintString` "iwork"))))

(event `self.trigger.OnComponentBeginOverlap`
  (params (OverlappedComponent :type "PrimitiveComponent Object Reference") (OtherActor :type "Actor Object Reference") (OtherComp :type "PrimitiveComponent Object Reference") (OtherBodyIndex :type Integer) (bFromSweep :type Boolean) (SweepResult :type "HitResult Structure (by ref)"))
  (bind _asbp_third_person_character_custom (cast `/Game/Blueprints/BP_ThirdPersonCharacterCustom` OtherActor))
  (set `/Game/Blueprints/BP_ThirdPersonCharacterCustom.KidCount` (+ (`/Game/Blueprints/BP_ThirdPersonCharacterCustom.KidCount` _asbp_third_person_character_custom) 1) _asbp_third_person_character_custom)
  (`|ExecutionSequence`
    (:`then_1`
      (`self.K2_DestroyActor`)
      (`KismetSystemLibrary.PrintString` "got Child" true true (struct :`G` 0.66 :`B` 1.0 :`A` 1.0) 5.0))))

(fn `UserConstructionScript`)