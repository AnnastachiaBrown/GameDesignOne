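; BP_Mother is a mother NPC whose response on capsule overlap depends on the player character's KidCount.
; At one or below it shows timed texts and adds a key; at exactly two, the child delivery, it hides CoinText and adds money.
; Higher counts show failure text, then play the MotherFallingApart timeline, whose update snaps the head to HeadEnd's relative location with sweep and hides that text.
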(event `self.Capsule.OnComponentBeginOverlap`
  (params (OverlappedComponent :type "PrimitiveComponent Object Reference") (OtherActor :type "Actor Object Reference") (OtherComp :type "PrimitiveComponent Object Reference") (OtherBodyIndex :type Integer) (bFromSweep :type Boolean) (SweepResult :type "HitResult Structure (by ref)"))
  (bind _asbp_third_person_character_custom (cast `/Game/Blueprints/BP_ThirdPersonCharacterCustom` OtherActor))
  (bind _kidcount (`/Game/Blueprints/BP_ThirdPersonCharacterCustom.KidCount` _asbp_third_person_character_custom))
  (if (<= _kidcount 1)
    ;[1 1 1] First Interaction With Mother
    (`SceneComponent.SetVisibility` (`self.InformationText`) true false)
    (`KismetSystemLibrary.Delay` 4.5)
    (`SceneComponent.SetVisibility` (`self.InformationText`) false false)
    (`KismetSystemLibrary.Delay` 0.2)
    (set `/Game/Blueprints/BP_ThirdPersonCharacterCustom.Key Count` (+ (`/Game/Blueprints/BP_ThirdPersonCharacterCustom.Key Count` _asbp_third_person_character_custom) 1) _asbp_third_person_character_custom)
    (`SceneComponent.SetVisibility` (`self.InformationText1`) true false)
    (`KismetSystemLibrary.PrintString` "Got KEY" true true (struct :`G` 0.66 :`B` 1.0 :`A` 1.0) 5.0)
    (`KismetSystemLibrary.Delay` 5.0)
    (`SceneComponent.SetVisibility` (`self.InformationText1`) false false)
    (elif (== _kidcount 2)
      ;[1 1 1] Bringing the child to the mother
      (`SceneComponent.SetVisibility` (`self.CoinText`) false false)
      (`KismetSystemLibrary.PrintString` "got 1 Coint")
      (set `/Game/Blueprints/BP_ThirdPersonCharacterCustom.moneyCount` (+ (`/Game/Blueprints/BP_ThirdPersonCharacterCustom.moneyCount` _asbp_third_person_character_custom) 1) _asbp_third_person_character_custom)
      (`KismetSystemLibrary.Delay` 5.0)
      (else
        (`SceneComponent.SetVisibility` (`self.FailureText`) true false)
        (`KismetSystemLibrary.Delay` 3.0)
        (`Timeline|MotherFallingApart`
          (:`Update`
            (`SceneComponent.K2_SetRelativeLocation` (`self.Head`) (`SceneComponent.RelativeLocation` (`self.Head End`)) true false)
            (`SceneComponent.SetVisibility` (`self.FailureText`) false false)))))))

(fn `UserConstructionScript`)