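; BP_CircusMan is a circus NPC actor that gives timed dialogue for a find-the-kid quest when the player overlaps its Trigger.
; The player character's KidCount selects the branch, each toggling components' visibility between delays.
; Low counts show circus info; two shows the got-kid lines, pays coins, increments KidCount and prints a hint to tell the mother.
; Higher counts show NoChild, then destroy the actor.
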(event `self.Trigger.OnComponentBeginOverlap`
  (params (OverlappedComponent :type "PrimitiveComponent Object Reference") (OtherActor :type "Actor Object Reference") (OtherComp :type "PrimitiveComponent Object Reference") (OtherBodyIndex :type Integer) (bFromSweep :type Boolean) (SweepResult :type "HitResult Structure (by ref)"))
  (bind _asbp_third_person_character_custom (cast `/Game/Blueprints/BP_ThirdPersonCharacterCustom` OtherActor))
  (bind _kidcount (`/Game/Blueprints/BP_ThirdPersonCharacterCustom.KidCount` _asbp_third_person_character_custom))
  (if (<= _kidcount 1)
    (`SceneComponent.SetVisibility` (`self.CircusInfo`) true false)
    (`KismetSystemLibrary.Delay` 3.0)
    (`SceneComponent.SetVisibility` (`self.CircusInfo`) false false)
    (`SceneComponent.SetVisibility` (`self.CircusInfo1`) true false)
    (`KismetSystemLibrary.Delay` 5.0)
    (`SceneComponent.SetVisibility` (`self.CircusInfo1`) false false)
    (elif (== _kidcount 2)
      (`SceneComponent.SetVisibility` (`self.GotKid`) true false)
      (`KismetSystemLibrary.Delay` 5.0)
      (`SceneComponent.SetVisibility` (`self.GotKid`) false false)
      (`SceneComponent.SetVisibility` (`self.GotKid1`) true false)
      (set `/Game/Blueprints/BP_ThirdPersonCharacterCustom.moneyCount` (+ (`/Game/Blueprints/BP_ThirdPersonCharacterCustom.moneyCount` _asbp_third_person_character_custom) 5) _asbp_third_person_character_custom)
      (`KismetSystemLibrary.PrintString` "got 5 COINS" true true (struct :`G` 0.66 :`B` 1.0 :`A` 1.0) 5.0)
      (`KismetSystemLibrary.Delay` 5.0)
      (`SceneComponent.SetVisibility` (`self.GotKid1`) false false)
      (set `/Game/Blueprints/BP_ThirdPersonCharacterCustom.KidCount` (+ (`/Game/Blueprints/BP_ThirdPersonCharacterCustom.KidCount` _asbp_third_person_character_custom) 1) _asbp_third_person_character_custom)
      (`KismetSystemLibrary.PrintString` "go tell the mother" true true (struct :`G` 0.66 :`B` 1.0 :`A` 1.0) 5.0)
      (else
        (`SceneComponent.SetVisibility` (`self.NoChild`) true false)
        (`KismetSystemLibrary.Delay` 10.0)
        (`SceneComponent.SetVisibility` (`self.NoChild`) false false)
        (`KismetSystemLibrary.Delay` 10.0)
        (`self.K2_DestroyActor`)))))

(fn `UserConstructionScript`)