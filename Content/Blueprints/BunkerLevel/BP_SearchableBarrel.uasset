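; BP_SearchableBarrel is a searchable barrel in the bunker level that reports how many coins it holds.
; Its Trigger overlap shows or hides a Widget for the custom third-person character.
; The E key, not gated by that overlap in the graph, fires once to create a W_Dialouge with the found-coins text.
; It then calls RemoveAllWidgets without adding the dialogue to the viewport and zeroes CoinAmount, crediting no one.
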(event `Key|E`
  (params (Key :type "Key Structure"))
  (bind _coinamount (`self.CoinAmount`))
  (:`Pressed`
    (`/Engine/EditorBlueprintResources/StandardMacros.DoOnce` false
      (:`Completed`
        (bind _returnvalue (`|CreateWidget` "/Game/Widgets/emotionWidgets/W_Dialouge.W_Dialouge_C" (`GameplayStatics.GetPlayerController` 0)))
        (set `self.UI` _returnvalue)
        (`TextBlock.SetText` (`/Game/Widgets/emotionWidgets/W_Dialouge.TalkText` (`self.UI`)) (`KismetTextLibrary.Conv_StringToText` (`KismetStringLibrary.Concat_StrStr` "You Found " (`KismetStringLibrary.Conv_IntToString` (`self.CoinAmount`)) " Coins!")))
        (`WidgetLayoutLibrary.RemoveAllWidgets`)
        (set `self.CoinAmount` (- _coinamount _coinamount))))))

(event `self.Trigger.OnComponentBeginOverlap`
  (params (OverlappedComponent :type "PrimitiveComponent Object Reference") (OtherActor :type "Actor Object Reference") (OtherComp :type "PrimitiveComponent Object Reference") (OtherBodyIndex :type Integer) (bFromSweep :type Boolean) (SweepResult :type "HitResult Structure (by ref)"))
  (cast `/Game/Blueprints/BP_ThirdPersonCharacterCustom` OtherActor)
  (`SceneComponent.SetVisibility` (`self.Widget`) true false))

(event `self.Trigger.OnComponentEndOverlap`
  (params (OverlappedComponent :type "PrimitiveComponent Object Reference") (OtherActor :type "Actor Object Reference") (OtherComp :type "PrimitiveComponent Object Reference") (OtherBodyIndex :type Integer))
  (cast `/Game/Blueprints/BP_ThirdPersonCharacterCustom` OtherActor)
  (`SceneComponent.SetVisibility` (`self.Widget`) false false))

(fn `UserConstructionScript`)