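; BP_SearchableBarrel is a barrel the player can search once.
; Trigger overlaps with the custom third-person character show or hide a prompt widget while the barrel is unsearched.
; On interact, it marks itself searched, hides the prompt, opens the W_SearchableChests widget and switches to UI-only input with a mouse cursor.
; A Searched macro gates all three events on the Searched flag.
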(event `self.Trigger.OnComponentBeginOverlap`
  (params (OverlappedComponent :type "PrimitiveComponent Object Reference") (OtherActor :type "Actor Object Reference") (OtherComp :type "PrimitiveComponent Object Reference") (OtherBodyIndex :type Integer) (bFromSweep :type Boolean) (SweepResult :type "HitResult Structure (by ref)"))
  (`self.Searched`
    (:`true`
      (cast `/Game/Blueprints/BP_ThirdPersonCharacterCustom` OtherActor)
      (`SceneComponent.SetVisibility` (`self.Widget`) true false))))

(event `self.Trigger.OnComponentEndOverlap`
  (params (OverlappedComponent :type "PrimitiveComponent Object Reference") (OtherActor :type "Actor Object Reference") (OtherComp :type "PrimitiveComponent Object Reference") (OtherBodyIndex :type Integer))
  (`self.Searched`
    (:`true`
      (cast `/Game/Blueprints/BP_ThirdPersonCharacterCustom` OtherActor)
      (`SceneComponent.SetVisibility` (`self.Widget`) false false))))

(event `/Game/Blueprints/BunkerLevel/Searchables/BPI_Interactions.OnInteractBegin`
  (bind _returnvalue (`GameplayStatics.GetPlayerController` 0))
  (`self.Searched`
    (:`true`
      (set `self.Searched?` true)
      (`SceneComponent.SetVisibility` (`self.Widget`) false false)
      (bind _returnvalue_2 (`|CreateWidget` "/Game/Widgets/BunkerWidgets/W_SearchableChests.W_SearchableChests_C"))
      (`UserWidget.AddToViewport` _returnvalue_2 0)
      (`WidgetBlueprintLibrary.SetInputMode_UIOnlyEx` _returnvalue null)
      (set `PlayerController.bShowMouseCursor` true _returnvalue))))

(fn `UserConstructionScript`)