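; BP_Patrol_Ai is an AI pawn Blueprint that patrols between level actors tagged PatrolPoint.
; BeginPlay gathers and shuffles the points, then a self-recalling AI MoveTo event visits each in turn, advancing after a short delay on success or failure.
; The list reshuffles whenever a full loop completes.
; A separate looping event chases the first player character, but nothing in this Blueprint starts it.
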(event `self.ReceiveBeginPlay`
  (bind _outactors (`GameplayStatics.GetAllActorsOfClassWithTag` "/Script/Engine.Actor" "PatrolPoint"))
  (`KismetSystemLibrary.PrintString` (`KismetStringLibrary.Concat_StrStr` "there are " (`KismetStringLibrary.Conv_IntToString` (`KismetArrayLibrary.Array_Length` _outactors)) " Patrol Points") true true (struct :`G` 0.66 :`B` 1.0 :`A` 1.0) 5.0)
  (`KismetArrayLibrary.Array_Shuffle` _outactors)
  (`self.MoveTowardsPatralPoints`))

(event `MoveTowardsPatralPoints`
  ;[1 1 1] patrol
  (`|AIMoveTo` self (`self.K2_GetActorLocation` (`|GetArrayItem` (stale `self.ReceiveBeginPlay` _outactors) (`self.CurrentPatrolPoint`))) null 100.0
    (:`OnSuccess`
      (`KismetSystemLibrary.PrintString` "successPAtrol" true true (struct :`R` 0.552878 :`G` 1.0 :`B` 0.289342 :`A` 1.0)))
    (:`OnFail`
      (`KismetSystemLibrary.PrintString` "failed to patrol" true true (struct :`R` 1.0 :`G` 0.232179 :`B` 0.140474 :`A` 1.0))))
  (bind _result (`/Engine/EditorBlueprintResources/StandardMacros.IncrementInt` (`self.CurrentPatrolPoint`))
    (:`  `
      (if (>= _result (`KismetArrayLibrary.Array_Length` (stale `self.ReceiveBeginPlay` _outactors)))
        (set `self.CurrentPatrolPoint` 0)
        (`KismetArrayLibrary.Array_Shuffle` (stale `self.ReceiveBeginPlay` _outactors)))
      (`KismetSystemLibrary.Delay` 1.0)
      (`self.MoveTowardsPatralPoints`))))

(event `movingTowardsPlayer`
  ;[1 1 1] move to player
  (`|AIMoveTo` self (0.0 0.0 0.0) (`GameplayStatics.GetPlayerCharacter` 0) 200.0
    (:`OnSuccess`
      (`KismetSystemLibrary.PrintString` "success" true true (struct :`R` 0.552878 :`G` 1.0 :`B` 0.289342 :`A` 1.0)))
    (:`OnFail`
      (`KismetSystemLibrary.PrintString` "failed to get to player" true true (struct :`R` 1.0 :`G` 0.232179 :`B` 0.140474 :`A` 1.0))))
  (`KismetSystemLibrary.Delay` 1.0)
  (`self.movingTowardsPlayer`))

(fn `UserConstructionScript`)