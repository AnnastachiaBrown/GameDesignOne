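; Actor component that adds an interactive dialogue to its owner, driven by a behavior tree.
; On BeginPlay it spawns a dedicated dialogue AI controller to run the tree.
; Interaction shows the dialogue widget, switches input to UI-only with a cursor, starts the tree and passes the widget through the blackboard.
; The widget's exit event stops the tree, removes the widget and restores game input.
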(event `self.ReceiveBeginPlay`
  (bind _returnvalue (`|SpawnActorFromClass` "/Game/Blueprints/BunkerLevel/Charecters/Dialouge/BP_DialougeAIController.BP_DialougeAIController_C" (`KismetMathLibrary.MakeTransform` (0.0 0.0 0.0)) "Undefined" "MultiplyWithRoot" null null))
  (set `self.AIController` _returnvalue))

(event `/Game/Blueprints/BunkerLevel/Charecters/Dialouge/BPI_Dialouge.OnInteraction`
  (params (PlayerCharecter :type "/Game/Blueprints/BP_ThirdPersonCharacterCustom Object Reference"))
  (bind _returnvalue (`GameplayStatics.GetPlayerController` 0))
  (bind _returnvalue_2 (`|GenericCreateObject` (cast `PlayerController` (`Pawn.GetController` PlayerCharecter) :!pure true) "/Game/Widgets/BunkerWidgets/W_AdvancedDialouge.W_AdvancedDialouge_C"))
  (bind _output_get (set `self.DialougeUI` _returnvalue_2))
  (add `/Game/Widgets/BunkerWidgets/W_AdvancedDialouge.OnExit` _output_get (delegate `OnExit`))
  (`UserWidget.AddToViewport` _returnvalue_2 0)
  (`WidgetBlueprintLibrary.SetInputMode_UIOnlyEx` _returnvalue _returnvalue_2)
  (set `PlayerController.bShowMouseCursor` true _returnvalue)
  (`AIController.RunBehaviorTree` (`self.AIController`) (`self.DialougTree`))
  (bind _blackboardcomponent (`AIController.UseBlackboard` (`self.AIController`) "/Game/Blueprints/BunkerLevel/Charecters/Dialouge/DialougeBlackBoard.DialougeBlackBoard"))
  (`BlackboardComponent.SetValueAsObject` _blackboardcomponent "DialogWiget" (`self.DialougeUI`)))

(event `OnExit`
  (bind _returnvalue (`GameplayStatics.GetPlayerController` 0))
  (`WidgetBlueprintLibrary.SetInputMode_GameOnly` _returnvalue)
  (set `PlayerController.bShowMouseCursor` false _returnvalue)
  (`BrainComponent.StopLogic` (`AIController.BrainComponent` (`self.AIController`)) "Dialouge Exited")
  (`Widget.RemoveFromParent` (`self.DialougeUI`)))