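; BP_FinishTimer is a finish-line trigger actor that times the player's laps.
; On BeginPlay it adds a W_FInishLineTimed widget to the viewport and starts a self-calling event that refreshes the current lap time every 0.1 seconds.
; When BP_ThirdPersonCharacterCustom overlaps the Trigger, it prints the lap duration and resets the timestamp.
; Times derive from real-time seconds minus the last timestamp.
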(event `self.ReceiveBeginPlay`
  (bind _returnvalue (`|CreateWidget` "/Game/Widgets/W_FInishLineTimed.W_FInishLineTimed_C"))
  (bind _output_get (set `self.uiTimer` _returnvalue))
  (`UserWidget.AddToViewport` _output_get 0)
  (`self.onScreenTimer`))

(event `onScreenTimer`
  (`TextBlock.SetText` (`/Game/Widgets/W_FInishLineTimed.Timer` (`self.uiTimer`)) (`KismetTextLibrary.Conv_StringToText` (`KismetStringLibrary.Concat_StrStr` "current lap: " (`KismetTextLibrary.Conv_TextToString` (`KismetTextLibrary.Conv_DoubleToText` (- (`GameplayStatics.GetRealTimeSeconds`) (`self.lastTimeStamp`)) "HalfToEven" false true 1 324 1 1)) " Seconds ")))
  (`KismetSystemLibrary.Delay` 0.1)
  (`self.onScreenTimer`))

(event `self.Trigger.OnComponentBeginOverlap`
  (params (OverlappedComponent :type "PrimitiveComponent Object Reference") (OtherActor :type "Actor Object Reference") (OtherComp :type "PrimitiveComponent Object Reference") (OtherBodyIndex :type Integer) (bFromSweep :type Boolean) (SweepResult :type "HitResult Structure (by ref)"))
  (cast `/Game/Blueprints/BP_ThirdPersonCharacterCustom` OtherActor)
  (`KismetSystemLibrary.PrintString` (`KismetStringLibrary.Concat_StrStr` "That lap took " (`KismetTextLibrary.Conv_TextToString` (`KismetTextLibrary.Conv_DoubleToText` (- (`GameplayStatics.GetRealTimeSeconds`) (`self.lastTimeStamp`)) "HalfToEven" false true 1 324 0 1)) " seconds!"))
  (set `self.lastTimeStamp` (`GameplayStatics.GetRealTimeSeconds`)))

(fn `UserConstructionScript`)